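; AI controller for patrolling guards that runs the Patrol behavior tree and reacts when it perceives the player.
; On BeginPlay it counts the pawn's PatrolRoute waypoints and seeds the blackboard with pawn and waypoint data.
; Player perception updates set the enemy key, or clear it and record suspicion and last-seen location when nothing is perceived, raising aim either way.
; It prints every perception update; an unwired focus-tracking block never runs.
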(event OnTargetPerceptionUpdated(AIPerception)
  (params (Actor :type Actor%20Object%20Reference) (Stimulus :type AI%20Stimulus%20Structure))
  (bind _blackbrd (Variables|Default|GetBlackbrd))
  (bind _returnvalue (Class|AIPerceptionSystem|GetSenseClassforStimulus Stimulus))
  (Development|PrintString (Utilities|String|Append "Guard " (Utilities|GetObjectName (Pawn|GetControlledPawn)) "  " (Utilities|GetClassDisplayName _returnvalue) "  " (Utilities|GetClassDisplayName (Utilities|GetClass Actor)) "  " (Utilities|GetDisplayName Actor)))
  (if (== Actor (Game|Player|GetPlayerPawn 0))
    (if (not (== (Utilities|Array|Length (Class|AIPerceptionComponent|GetCurrentlyPerceivedActors (Variables|Default|GetAIPerception))) 0))
      (AI|Components|Blackboard|SetValueasObject (Variables|Default|GetBlackbrd) (Variables|Default|GetEnemyName) Actor)
      (bind _asthird_person_bp (Utilities|Casting|CastToThirdPersonBP (Pawn|GetControlledPawn)))
      (Variables|/Game/NPC/Behavior/ThirdPersonBP.ThirdPersonBP_C|SetAiming _asthird_person_bp true)
      (else
        (AI|Components|Blackboard|SetValueasObject _blackbrd (Variables|Default|GetEnemyName) 0)
        (AI|Components|Blackboard|SetValueasBool _blackbrd (Variables|Default|GetSuspicionName) true)
        (AI|Components|Blackboard|SetValueasVector _blackbrd (Variables|Default|GetLastSeenLocationName) (.StimulusLocation (Utilities|Struct|BreakAIStimulus Stimulus)))
        (bind _asthird_person_bp_2 (Utilities|Casting|CastToThirdPersonBP (Pawn|GetControlledPawn)))
        (Variables|/Game/NPC/Behavior/ThirdPersonBP.ThirdPersonBP_C|SetAiming _asthird_person_bp_2 true)))))

(event EventBeginPlay
  (CallFunction|InitialSetup)
  (bind _blackboardcomponent (Class|AIController|UseBlackboard "/Game/NPC/AI/PatrolData.PatrolData"))
  (CallFunction|BlackboardSetup _blackboardcomponent)
  (AI|RunBehaviorTree "/Game/NPC/AI/Patrol.Patrol"))

(event EventTick
  (params (DeltaSeconds :type Float%20%28single-precision%29)))

(fn ConstructionScript)

(fn InitialSetup
  (bind _self self)
  (bind _returnvalue (Pawn|GetControlledPawn _self))
  (bind _returnvalue_2 (Actor|GetComponentbyClass _returnvalue "/Script/TestingGrounds.PatrolRoute"))
  (if (!= _returnvalue_2 0)
    (bind _returnvalue_3 (Class|PatrolRoute|GetPatrolPoints _returnvalue_2))
    (Variables|Default|SetNumberOfWaypoints (Utilities|Array|Length _returnvalue_3))))

(fn BlackboardSetup
  (params (Blackboard :type Blackboard%20Component%20Object%20Reference))
  (AI|Components|Blackboard|SetValueasObject Blackboard (Variables|Default|GetSelfActor%20Name) (Pawn|GetControlledPawn self))
  (Class|BlackboardComponent|SetValueasInt Blackboard (Variables|Default|GetNumberOfWaypoints%20Name) (Variables|Default|GetNumberOfWaypoints))
  (Class|BlackboardComponent|SetValueasInt Blackboard (Variables|Default|GetNextWaypointIndex%20Name))
  (Variables|Default|SetBlackbrd Blackboard))