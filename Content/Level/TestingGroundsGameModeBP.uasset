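; TestingGroundsGameModeBP is a game mode Blueprint that spawns the starting level tile at StartLocation on BeginPlay.
; An unconnected chain would spawn further tiles in a loop from StartingIndex toward NumberOfTiles, placing each at the previous tile's attach location.
; That loop never runs, so only the first tile is spawned here.
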(event EventBeginPlay
  (bind _returnvalue (Game|SpawnActorfromClass "/Game/Terrain/Tile.Tile_C" (Variables|Default|GetStart%20Location) "Undefined" self 0)))

(event EventTick
  (params (DeltaSeconds :type Float%20%28single-precision%29)))

(fn ConstructionScript)